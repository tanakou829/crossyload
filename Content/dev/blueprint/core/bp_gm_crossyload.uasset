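; Game mode for a Crossy Road-style game that tracks the player's position on a grid and keeps the field informed of it.
; On BeginPlay it casts player character 0 to the crossyload player, binds to its four directional move dispatchers and spawns the field actor.
; Move handlers shift the stored 2D location by one step, with X as forward and Y as right, then pass it to the field's location event.
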(event Custom|event_move_front_event
  ;[1 1 1] change_potision
  (CallFunction|AddPosition 0 1)
  (Default|FieldLocationEventEvent (Variables|Default|Getfield_object) (Variables|Default|Getcharacter_location)))

(event Custom|event_move_back_event
  ;[1 1 1] change_potision
  (CallFunction|AddPosition 0 -1)
  (Default|FieldLocationEventEvent (Variables|Default|Getfield_object) (Variables|Default|Getcharacter_location)))

(event Custom|event_move_right_event
  ;[1 1 1] change_potision
  (CallFunction|AddPosition 1)
  (Default|FieldLocationEventEvent (Variables|Default|Getfield_object) (Variables|Default|Getcharacter_location)))

(event Custom|event_move_left_event
  ;[1 1 1] change_potision
  (CallFunction|AddPosition -1)
  (Default|FieldLocationEventEvent (Variables|Default|Getfield_object) (Variables|Default|Getcharacter_location)))

(event EventBeginPlay
  ;[1 1 1] crossy playerのcast
  (bind _asbp_crossyload_player (Utilities|Casting|CastTobp_crossyload_player (Game|GetPlayerCharacter 0)))
  (Variables|Default|SetAs%20Bp%20Crossyload%20Player _asbp_crossyload_player)
  ;[1 1 1] move
  (EventDispatchers|AssignEventMoveFront (Variables|Default|GetAs%20Bp%20Crossyload%20Player) (EventDispatchers|CreateEvent :!event Custom|event_move_front_event))
  (EventDispatchers|AssignEventMoveBack (Variables|Default|GetAs%20Bp%20Crossyload%20Player) (EventDispatchers|CreateEvent :!event Custom|event_move_back_event))
  (EventDispatchers|AssignEventMoveRight (Variables|Default|GetAs%20Bp%20Crossyload%20Player) (EventDispatchers|CreateEvent :!event Custom|event_move_right_event))
  (EventDispatchers|AssignEventMoveLeft (Variables|Default|GetAs%20Bp%20Crossyload%20Player) (EventDispatchers|CreateEvent :!event Custom|event_move_left_event))
  (bind _returnvalue (Game|SpawnActorfromClass "/Game/dev/blueprint/actor/bp_field.bp_field_C" (Math|Transform|MakeTransform "0, 0, 0" "0, 0, 0" "1.000000,1.000000,1.000000") "Undefined" "MultiplyWithRoot" 0 0))
  (Variables|Default|Setfield_object _returnvalue))

(fn ConstructionScript)

(fn AddPosition
  (params (right_move :type Integer) (front_move :type Integer))
  (Variables|Default|Setcharacter_location (Utilities|Struct|Makevector2d_int (+ (.x (Variables|Default|Getcharacter_location)) front_move) (+ right_move (.y (Variables|Default|Getcharacter_location))))))