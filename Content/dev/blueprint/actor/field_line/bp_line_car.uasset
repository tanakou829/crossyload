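; Road lane actor for a field line that runs one obstacle car across itself at a time.
; On BeginPlay a random-delay timer starts to spawn a bp_obstract_car at the left spawn point, attached to the lane root.
; Tick moves the car by a fixed local Y step, not scaled by delta time.
; Either trigger box destroys cars that overlap it, and the car's OnDestroyed restarts the timer.
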(event OnComponentBeginOverlap(Box)
  (params (OverlappedComponent :type Primitive%20Component%20Object%20Reference) (OtherActor :type Actor%20Object%20Reference) (OtherComp :type Primitive%20Component%20Object%20Reference) (OtherBodyIndex :type Integer) (bFromSweep :type Boolean) (SweepResult :type Hit%20Result%20Structure%20%28by%20ref%29))
  (bind _asbp_obstract_car (Utilities|Casting|CastTobp_obstract_car OtherActor))
  (Actor|DestroyActor _asbp_obstract_car))

(event OnComponentBeginOverlap(Box1)
  (params (OverlappedComponent :type Primitive%20Component%20Object%20Reference) (OtherActor :type Actor%20Object%20Reference) (OtherComp :type Primitive%20Component%20Object%20Reference) (OtherBodyIndex :type Integer) (bFromSweep :type Boolean) (SweepResult :type Hit%20Result%20Structure%20%28by%20ref%29))
  (bind _asbp_obstract_car (Utilities|Casting|CastTobp_obstract_car OtherActor))
  (Actor|DestroyActor _asbp_obstract_car))

(event Custom|spawn_car
  (bind _returnvalue (Game|SpawnActorfromClass "/Game/dev/blueprint/actor/obstacle/bp_obstract_car.bp_obstract_car_C" (Transformation|GetRelativeTransform (Variables|Default|Getcar_spawn_point_left)) "Undefined" "MultiplyWithRoot" 0 0))
  (Transformation|AttachComponentToComponent _returnvalue (Variables|Default|GetDefaultSceneRoot) "None" "KeepRelative" "KeepRelative" "KeepRelative" true)
  (Variables|Default|Setcurrent_car _returnvalue)
  (Game|AssignOnDestroyed (Variables|Default|Getcurrent_car) (delegate Custom|OnDestroyed_event)))

(event Custom|spawn_car_event
  (Utilities|Time|SetTimerbyEvent (EventDispatchers|CreateEvent :!event Custom|spawn_car) (Math|Random|RandomFloatinRange 1.0 5.0)))

(event Custom|OnDestroyed_event
  (params (DestroyedActor :type Actor%20Object%20Reference))
  (CallFunction|SpawnCarEvent))

(event EventBeginPlay
  (|CallParentFunction)
  (CallFunction|SpawnCarEvent))

(event Collision|EventActorBeginOverlap
  (params (OtherActor :type Actor%20Object%20Reference))
  (|CallParentFunction OtherActor) ; このノードは無効になっているため呼び出せません。\n機能をビルドするにはピンをドラッグしてください。
)

(event EventTick
  (params (DeltaSeconds :type Float%20%28single-precision%29))
  (Utilities|IsValid (Variables|Default|Getcurrent_car)
    (:Is%20Valid
      (Transformation|AddActorLocalOffset (Variables|Default|Getcurrent_car) "0.000000,40.000000,0.000000" false false))))

(fn ConstructionScript
  (|CallParentFunction))