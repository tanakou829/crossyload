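; Field manager actor that builds a strip of random car and field lines at BeginPlay and scrolls it as a whole.
; Lines are placed along X by their accumulated widths, stored in an array and attached to a shared Locator component.
; On each field location event, a timeline lerps the Locator's X and Y to the negated, scaled location, moving the world opposite to that position.
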(event Custom|field_location_event_Event
  (params (NewParam :type Vector%202d%20Int%20Structure))
  (bind (_x _y) (Utilities|Struct|Breakvector2d_int NewParam))
  (Variables|Default|SetRelative%20Location (Variables|/Script/Engine.SceneComponent|GetRelativeLocation (Variables|Default|Getlocator)))
  (bind _blend (Timeline|タイムライン PlayFromStart)
    (:Update
      (Transformation|SetRelativeLocation (Variables|Default|Getlocator) (Math|Vector|MakeVector (Math|Float|Lerp (.x (Variables|Default|GetRelative%20Location)) (* (Math|Conversions|ToFloat(Integer) (* _x 100)) -1.0) _blend) (Math|Float|Lerp (.y (Variables|Default|GetRelative%20Location)) (* (Math|Conversions|ToFloat(Integer) (* _y 100)) -1.0) _blend) 0.0) false false))))

(event Custom|initialize_line
  (for _index (range -10 10)
    (bind _returnvalue (Game|SpawnActorfromClass (.OutItem (Utilities|Array|Random (Utilities|Array|MakeArray "/Game/dev/blueprint/actor/field_line/bp_line_car.bp_line_car_C" "/Game/dev/blueprint/actor/field_line/bp_field_line.bp_field_line_C"))) (Math|Transform|MakeTransform "0, 0, 0" "0, 0, 0" "1.000000,1.000000,1.000000") "Undefined" "MultiplyWithRoot" 0 0))
    (bind _asbp_field_line_base (Utilities|Casting|CastTobp_field_line_base _returnvalue))
    (Transformation|SetActorLocation _asbp_field_line_base (Math|Vector|MakeVector (Variables|Default|Getall_width) 0.0 0.0) false true)
    (Variables|Default|Setall_width (+ (Variables|Default|Getall_width) (Variables|/Game/dev/blueprint/actor/field_line/bp_field_line_base.bp_field_line_base_C|Getwidth _asbp_field_line_base)))
    (Utilities|Array|Add (Variables|Default|Getfield_line_actors) _returnvalue)
    (Transformation|AttachComponentToComponent _returnvalue (Variables|Default|Getlocator) "None" "KeepRelative" "KeepRelative" "KeepRelative" true)))

(event EventBeginPlay
  (EventDispatchers|BindEventtoFieldLocationEvent (delegate Custom|field_location_event_Event))
  (CallFunction|InitializeLine))

(fn ConstructionScript)